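; SpriteCharacter is a character Blueprint that exposes a name and a set of expressions.
; Getter functions return the raw Name, a display name converted from it to text, and the current expression.
; The supported expressions come from the keys of the Expressions map, so that map defines which expressions the character offers.
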(fn GetDisplayName
  (return (Utilities|Text|ToText(Name) (Variables|Default|GetName))))

(fn GetExpression
  (return (Variables|Default|GetCurrentExpression)))

(fn GetName
  (return (Variables|Default|GetName)))

(fn GetSupportedExpressions
  (bind _keys (Utilities|Map|Keys (Variables|Default|GetExpressions)))
  (return _keys))